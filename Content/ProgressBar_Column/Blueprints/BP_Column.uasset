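; BP_Column is a VR button column where repeated presses fill a progress bar widget before it drains empty.
; Tick projects motion controller movement onto the button's up axis, increments the bar at full depth, then interpolates the button back.
; The AutoDecresisng timeline drains the bar with sound, showing text and disabling the column at zero.
; A full bar stops the drain, raises WinPlane, hides the widget and opens a video.
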(event `self.ReceiveBeginPlay`
  ;[0.6511 1 0.5885] Создаем и запоминаем Widget с Progress Bar-ом
  (bind _returnvalue (`|CreateWidget` "/Game/ProgressBar_Column/WBP/WBP_ProgressBar.WBP_ProgressBar_C"))
  (set `self.Reference To WBP_ProgressBar` _returnvalue))

(event `self.VR_Button.OnComponentBeginOverlap`
  (params (OverlappedComponent :type "PrimitiveComponent Object Reference") (OtherActor :type "Actor Object Reference") (OtherComp :type "PrimitiveComponent Object Reference") (OtherBodyIndex :type Integer) (bFromSweep :type Boolean) (SweepResult :type "HitResult Structure (by ref)"))
  ;[0.6511 1 0.5885] По касанию получаем начальные координаты кнопки и контроллера игрока
  (bind _asbp_motion_controller (cast `/Game/VirtualRealityBP/Blueprints/BP_MotionController` OtherActor))
  (set `self.Ref_ToMotionController` (`/Game/VirtualRealityBP/Blueprints/BP_MotionController.MotionController` _asbp_motion_controller))
  (if (not (`self.b_returning`))
    (set `self.b_istouching?` true)
    (set `self.Start_MotionControllerLocation` (`SceneComponent.K2_GetComponentLocation` (`self.Ref_ToMotionController`))) ; Положение контроллера
    (set `self.StartButtonLocation` (`SceneComponent.K2_GetComponentLocation` (`self.VR_Button`)))))

(event `self.ReceiveTick`
  (params (DeltaSeconds :type "Float (single-precision)"))
  (bind _vr_button (`self.VR_Button`))
  ;[0.6511 1 0.5885] Проверка условий для взаимодействия с кнопкой по Tick
  (set `self.delta sec` DeltaSeconds)
  (if (`self.b_isbroken?`)
    _
    (elif (>= (`/Game/ProgressBar_Column/WBP/WBP_ProgressBar.ProgressBarValue` (`self.Reference To WBP_ProgressBar`)) 1.0)
      ;[0.6511 1 0.5885] Progress bar заполнен
      (`/Engine/EditorBlueprintResources/StandardMacros.DoOnce` false
        (:`Completed`
          (`self.Progress bar is Full!`)
          (`self.MakeWinPlatform`) ; Выполняем событие на подъем платформы
        ))
      (else
        (`WidgetComponent.SetWidget` (`self.Widget`) (`self.Reference To WBP_ProgressBar`))
        (if (`self.b_istouching?`)
          ;[0.6511 1 0.5885] Кнопка нажимается игроком
          (set `self.ButtonMovement` (`KismetMathLibrary.FClamp` (`KismetMathLibrary.VSize` (`KismetMathLibrary.ProjectVectorOnToVector` (- (`SceneComponent.K2_GetComponentLocation` (`self.Ref_ToMotionController`)) (`self.Start_MotionControllerLocation`)) (`SceneComponent.GetUpVector` (`self.VR_Button`)))) 0.0 (`self.MaxButtonDisplacement`))) ; Сдвиг кнопки по оси Z
          (bind _output_get (set `self.EndButtonLocation` (- (`self.StartButtonLocation`) (* (`SceneComponent.GetUpVector` _vr_button) (`self.ButtonMovement`)))))
          (`SceneComponent.K2_SetWorldLocation` _vr_button _output_get false false) ; Устанвливаем положение кнопки
          (if (>= (`self.ButtonMovement`) (`self.MaxButtonDisplacement`))
            (set `self.b_istouching?` false) ; Теперь мы игнорируем касания игрока
            (set `self.b_returning` true) ; Теперь кнопка возвращается в изначальное положение
            (`/Game/ProgressBar_Column/WBP/WBP_ProgressBar.Increasse progress bar` (`self.Reference To WBP_ProgressBar`)) ; Вызываем функцию увеличение Progress Bar-a в Widgete
            (`PrimitiveComponent.SetMaterial` (`self.VR_Button`) 0 "/Game/ProgressBar_Column/Material/M_ButtonRelesed.M_ButtonRelesed") ; Устанавливаем материал
            (`GameplayStatics.PlaySound2D` "/Engine/VREditor/Sounds/UI/Gizmo_Handle_Clicked.Gizmo_Handle_Clicked" 1.0 1.0 0.0 null null) ; Звук кнопки
          )
          (else
            ;[0.6511 1 0.5885] Кнопка возвращается обратно
            (if (`self.b_returning`)
              (bind _output_get_2 (set `self.EndButtonLocation` (`KismetMathLibrary.VInterpTo` (`self.EndButtonLocation`) (`self.StartButtonLocation`) (`GameplayStatics.GetWorldDeltaSeconds`) (`self.ButtonreturnSpeed`)))) ; Устанавливаем конечное положение кнопки равное начальному
              (`SceneComponent.K2_SetWorldLocation` (`self.VR_Button`) _output_get_2 false false) ; Возвращаем кнопку на место
              (if (`KismetMathLibrary.EqualExactly_VectorVector` (`self.EndButtonLocation`) (`self.StartButtonLocation`))
                (set `self.b_returning` false) ; Теперь кнопка не возвращается
                (`PrimitiveComponent.SetMaterial` (`self.VR_Button`) 0 "/Game/ProgressBar_Column/Material/M_ButtonPressed.M_ButtonPressed")))))))))

(event `Progress bar is Full!`
  (bind _reference_to_wbp_progressbar (`self.Reference To WBP_ProgressBar`))
  ;[0.6511 1 0.5885] Уменьшаем Progress Bar по Таймлайну раз в 1 секунду
  (`Timeline|Auto Decresisng` :!via `Stop`
    (:`NewTrack_0`
      (`/Game/ProgressBar_Column/WBP/WBP_ProgressBar.Decrease progress bar` _reference_to_wbp_progressbar) ; Уменьшаем значения Progress Bar
      (`GameplayStatics.PlaySound2D` "/Engine/VREditor/Sounds/UI/Dockable_Window_Close.Dockable_Window_Close" 1.0 1.0 0.0 null null) ; Звук уменьшения значения Progress Bar
      (if (<= (`/Game/ProgressBar_Column/WBP/WBP_ProgressBar.ProgressBarValue` _reference_to_wbp_progressbar) 0.0)
        (`self.Progress bar is Full!`) ; Выключаем этот таймлайн
        (`GameplayStatics.PlaySound2D` "/Engine/VREditor/Sounds/VR_click3.VR_click3" 1.0 1.0 0.0 null null)
        (`SceneComponent.SetVisibility` (`self.TextRender`) true false)
        (set `self.b_isbroken?` true)))))

(event `MakeWinPlatform`
  ;[0.6511 1 0.5885] Поднимаем платформу
  (bind (_direction _timeline_for_video_plane_creation) (`Timeline|Подъем платформы 3 секунды` :!via `PlayFromStart`)
    (:`Update`
      (`SceneComponent.K2_SetRelativeLocation` (`self.Win_Plane`) (`KismetMathLibrary.VLerp` (`SceneComponent.RelativeLocation` (`self.Win_Plane`)) (`self.EndLocation for video`) _timeline_for_video_plane_creation) false false) ; Меня положение платформы
      (`SceneComponent.SetVisibility` (`self.Widget`) false false))
    (:`Finished`
      (`MediaPlayer.OpenSource` (`self.MediaPlayer`) "/Game/Movies/Brian_Griffin_-_Never_Gonna_Give_You_Up.Brian_Griffin_-_Never_Gonna_Give_You_Up") ; Играем видео ,когда подняли платформу
    )))

(fn `UserConstructionScript`)